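; Player character Blueprint that reports health changes to the player's HUD.
; OnHealthChanged casts the controller to PlayerController_BP and sets the GlassBallWBP widget in its PrimaryUI to the ratio of health to max health.
; All other events are disabled stubs, and the construction script only calls its parent.
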(event `self.BP_OnHealthChanged`
  (params (Health :type "Float (single-precision)") (MaxHealth :type "Float (single-precision)"))
  (bind _asplayer_controller_bp (cast `/Game/Blueprints/PlayerController_BP` (`self.GetController`)))
  (`/Game/UI/GlassBall_WBP.SetPercentage` (`/Game/UI/PrimaryUI_WBP.GlassBall_WBP` (`/Game/Blueprints/PlayerController_BP.PrimaryUI` _asplayer_controller_bp)) (/ Health MaxHealth)))

(fn `UserConstructionScript`
  (`parent.UserConstructionScript`))