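; Player controller that creates the primary UI and translates player input into actions on the controlled pawn.
; On BeginPlay it creates the PrimaryUI_WBP widget, stores it and adds it to the viewport.
; Movement follows the camera's forward and right vectors, while look axes feed pitch and yaw input.
; Jump casts the pawn to Character, and the primary action casts it to CharacterBase_BP to trigger a melee attack.
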(event `self.ReceiveBeginPlay`
  (bind _returnvalue (`|CreateWidget` "/Game/UI/PrimaryUI_WBP.PrimaryUI_WBP_C"))
  (bind _output_get (set `self.PrimaryUI` _returnvalue))
  (`UserWidget.AddToViewport` _returnvalue 0)
  (`UserWidget.AddToViewport` _output_get 0))

(event `InputAxis|MoveForward`
  (params (AxisValue :type "Float (single-precision)"))
  ;[1 1 1] Basic Controls
  (`Pawn.AddMovementInput` (`self.K2_GetPawn`) (`KismetMathLibrary.GetForwardVector` (`PlayerCameraManager.GetCameraRotation` (`self.PlayerCameraManager`))) AxisValue false))

(event `InputAxis|MoveRight`
  (params (AxisValue :type "Float (single-precision)"))
  ;[1 1 1] Basic Controls
  (`Pawn.AddMovementInput` (`self.K2_GetPawn`) (`KismetMathLibrary.GetRightVector` (`PlayerCameraManager.GetCameraRotation` (`self.PlayerCameraManager`))) AxisValue false))

(event `InputAction|Jump`
  (params (Key :type "Key Structure"))
  ;[1 1 1] Basic Controls
  (:`Pressed`
    (bind _ascharacter (cast `Character` (`self.K2_GetPawn`)))
    (`Character.Jump` _ascharacter)))

(event `InputAxis|LookingUp`
  (params (AxisValue :type "Float (single-precision)"))
  ;[1 1 1] Basic Controls
  (`self.AddPitchInput` AxisValue))

(event `InputAxis|LookingRight`
  (params (AxisValue :type "Float (single-precision)"))
  ;[1 1 1] Basic Controls
  (`self.AddYawInput` AxisValue))

(event `InputAction|PrimaryAction`
  (params (Key :type "Key Structure"))
  (:`Pressed`
    (bind _ascharacter_base_bp (cast `/Game/Blueprints/Characters/CharacterBase_BP` (`self.K2_GetPawn`)))
    (`/Game/Blueprints/Characters/CharacterBase_BP.MeleeAttack` _ascharacter_base_bp)))

(fn `UserConstructionScript`)